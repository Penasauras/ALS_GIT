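; Base weapon Blueprint for a gun system, handling automatic fire and hitscan traces through the Advanced Locomotion System camera.
; StartShooting opens a gate that loops on a retriggerable fire-rate delay while ammo remains; StopShooting closes it.
; Each shot traces forward from the camera behavior component, but hits are not processed yet.
; Only the auto-fire branch is implemented, and the construction script fills WeaponData with the weapon's class.
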(event `self.ReceiveBeginPlay`
  (`self.OnBeginPlay`))

(event `StartShooting`
  (if (`self.HasAmmo?`)
    (if (`self.IsAutoFire`)
      (`|ExecutionSequence`
        (:`then_0`
          (`|ExecutionSequence`
            (:`then_0`
              (goto _label :!via `Open`))
            (:`then_1`
              (`/Engine/EditorBlueprintResources/StandardMacros.Gate` true :!label _label
                (:`Exit`
                  (`|ExecutionSequence`
                    (:`then_0`
                      (`KismetSystemLibrary.RetriggerableDelay` (`.FireRate_11_7AF2242C48079D05E7F45DB235BDE5E6` (break `/Game/Game/Data/Struct/WeaponData` (`self.WeaponData`))))
                      (if (`self.HasAmmo?`)
                        (goto _label)))
                    (:`then_1`
                      (`self.LineTraceForBullets`))))))))
        (:`then_1`
          (set `self.IsShooting?` true))))))

(event `StopShooting`
  (if (`self.HasAmmo?`)
    (`|ExecutionSequence`
      (:`then_0`
        (set `self.IsShooting?` false)
        (`|ExecutionSequence`
          (:`then_0`
            (goto _label :!via `Close`))))
      (:`then_1`
        (`SkeletalMeshComponent.Stop` (`self.WeaponMesh`))))))

(fn `LineTraceForBullets`
  (bind _camerabehavior (`/Game/AdvancedLocomotionV4/Blueprints/CameraSystem/ALS_PlayerCameraManager.CameraBehavior` (`self.Player Camera Manager`)))
  (bind _returnvalue (`SceneComponent.K2_GetComponentLocation` _camerabehavior))
  (bind (_outhit _returnvalue_2) (`KismetSystemLibrary.LineTraceSingle` _returnvalue (+ _returnvalue (* (`KismetMathLibrary.GetForwardVector` (`SceneComponent.K2_GetComponentRotation` _camerabehavior)) (`.TraceDistance_13_CCC4F1594E5FBA0D4E308CB4576FB619` (break `/Game/Game/Data/Struct/WeaponData` (`self.WeaponData`))))) "TraceTypeQuery1" false (`|MakeArray` (`self.Player REF`) (`GameplayStatics.GetPlayerCharacter` 0) :!type "Actor Object Reference") (`self.Draw Debug Type`)))
  (if _returnvalue_2
    _))

(fn `OnBeginPlay`
  (bind _asals_player_camera_manager (cast `/Game/AdvancedLocomotionV4/Blueprints/CameraSystem/ALS_PlayerCameraManager` (`GameplayStatics.GetPlayerCameraManager` 0)))
  (set `self.Player Camera Manager` _asals_player_camera_manager))

(fn `UserConstructionScript`
  (bind (_weapondata_currentweapontype _weapondata_class _weapondata_firerate _weapondata_tracedistance) (break `/Game/Game/Data/Struct/WeaponData` (`self.WeaponData`)))
  (set `self.WeaponData` (make `/Game/Game/Data/Struct/WeaponData` _weapondata_currentweapontype (`GameplayStatics.GetObjectClass` self) _weapondata_firerate _weapondata_tracedistance)))